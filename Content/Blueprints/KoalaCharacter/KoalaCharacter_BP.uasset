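; Koala player character Blueprint that handles the HUD, pause menu and tutorial screens.
; On begin play it attaches a BackplantPulp to the head socket; GameStarted adds a transparent HUD, plus the first tutorial in level 1.
; P toggles pause, swapping input mode, cursor and HUD visibility.
; Zone events clear old tutorial widgets and show the next of six screens, while progress events forward to those screens.
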(event Custom|RemoveTutorialWidgets
  (Utilities|FlowControl|Sequence
    (:then_0
      (if (not (Variables|/Game/Blueprints/PopUpScreens/FirstTutorialScreen.FirstTutorialScreen_C|GetbRemoved (Variables|Default|GetTutorialScreen)))
        (Widget|RemovefromParent (Variables|Default|GetTutorialScreen))))
    (:then_1
      (Utilities|IsValid (Variables|Default|GetSecondTutorialScreen)
        (:Is%20Valid
          (Widget|RemovefromParent (Variables|Default|GetSecondTutorialScreen)))))
    (:then_2
      (Utilities|IsValid (Variables|Default|GetThirdTutorialScreen)
        (:Is%20Valid
          (Widget|RemovefromParent (Variables|Default|GetThirdTutorialScreen)))))
    (:then_3
      (Utilities|IsValid (Variables|Default|GetFourthTutorialScreen)
        (:Is%20Valid
          (Widget|RemovefromParent (Variables|Default|GetFourthTutorialScreen)))))
    (:then_4
      (Utilities|IsValid (Variables|Default|GetFifthTutorialScreen)
        (:Is%20Valid
          (Widget|RemovefromParent (Variables|Default|GetFifthTutorialScreen)))))
    (:then_5
      (Utilities|IsValid (Variables|Default|GetSixthTutorialScreen)
        (:Is%20Valid
          (Widget|RemovefromParent (Variables|Default|GetSixthTutorialScreen)))))))

(event EventTextAdvance
  (bind _sixthtutorialscreen (Variables|Default|GetSixthTutorialScreen))
  (bind _secondtutorialscreen (Variables|Default|GetSecondTutorialScreen))
  (bind _tutorialscreen (Variables|Default|GetTutorialScreen))
  (bind _thirdtutorialscreen (Variables|Default|GetThirdTutorialScreen))
  (bind _fourthtutorialscreen (Variables|Default|GetFourthTutorialScreen))
  (bind _fifthtutorialscreen (Variables|Default|GetFifthTutorialScreen))
  (Utilities|FlowControl|Sequence
    (:then_0
      (Utilities|IsValid _tutorialscreen
        (:Is%20Valid
          (Default|CallAdvanceText _tutorialscreen))))
    (:then_1
      (Utilities|IsValid _secondtutorialscreen
        (:Is%20Valid
          (Default|CallAdvanceText _secondtutorialscreen))))
    (:then_2
      (Utilities|IsValid _thirdtutorialscreen
        (:Is%20Valid
          (Default|CallAdvanceText _thirdtutorialscreen))))
    (:then_3
      (Utilities|IsValid _fourthtutorialscreen
        (:Is%20Valid
          (Default|CallAdvanceText _fourthtutorialscreen))))
    (:then_4
      (Utilities|IsValid _fifthtutorialscreen
        (:Is%20Valid
          (Default|CallAdvanceText _fifthtutorialscreen))))
    (:then_5
      (Utilities|IsValid _sixthtutorialscreen
        (:Is%20Valid
          (Default|CallAdvanceText _sixthtutorialscreen))))))

(event EventBeginPlay
  (bind _returnvalue (Game|SpawnActorfromClass "/Game/Blueprints/KoalaCharacter/Assets/Placeholders/Backplant/BackplantPulp.BackplantPulp_C" (Math|Transform|MakeTransform "0, 0, 0" "0, 0, 0" "1,1,1") "Undefined" 0 0))
  (Transformation|AttachComponentToComponent _returnvalue (Variables|Character|GetMesh) "HeadSocket" "SnapToTarget" "SnapToTarget" "KeepRelative" true))

(event EventGameStarted
  (Input|SetInputModeGameOnly (Game|GetPlayerController 0))
  (bind _returnvalue (UserInterface|CreateWidget "/Game/Blueprints/HUD/KoalaHUD.KoalaHUD_C"))
  (bind _output_get (Variables|Default|SetHUD _returnvalue))
  (Widget|SetRenderOpacity _output_get 0.0)
  (UserInterface|Viewport|AddtoViewport (Variables|Default|GetHUD) 0)
  (if (== (Variables|Default|GetCurrentLevel) 1)
    (bind _returnvalue_2 (UserInterface|CreateWidget "/Game/Blueprints/PopUpScreens/FirstTutorialScreen.FirstTutorialScreen_C"))
    (bind _output_get_2 (Variables|Default|SetTutorialScreen _returnvalue_2))
    (UserInterface|Viewport|AddtoViewport _output_get_2 0)))

(event EventAxesRegistryFinished
  (bind _tutorialscreen (Variables|Default|GetTutorialScreen))
  (Utilities|IsValid _tutorialscreen
    (:Is%20Valid
      (Default|CallAxesRegistry _tutorialscreen))))

(event EventSeedGrowthStarted
  (bind _tutorialscreen (Variables|Default|GetTutorialScreen))
  (Utilities|IsValid _tutorialscreen
    (:Is%20Valid
      (Default|CallSeedGrowing _tutorialscreen))))

(event EventEnteredObstacleZone
  (CallFunction|RemoveTutorialWidgets)
  (bind _returnvalue (UserInterface|CreateWidget "/Game/Blueprints/PopUpScreens/SecondTutorialScreen.SecondTutorialScreen_C"))
  (bind _output_get (Variables|Default|SetSecondTutorialScreen _returnvalue))
  (UserInterface|Viewport|AddtoViewport _output_get 0))

(event EventObstacleZoneCompleted
  (CallFunction|RemoveTutorialWidgets)
  (bind _returnvalue (UserInterface|CreateWidget "/Game/Blueprints/PopUpScreens/ThirdTutorialScreen.ThirdTutorialScreen_C"))
  (bind _output_get (Variables|Default|SetThirdTutorialScreen _returnvalue))
  (UserInterface|Viewport|AddtoViewport _output_get 0))

(event EventEnteredShootingRange
  (CallFunction|RemoveTutorialWidgets)
  (bind _returnvalue (UserInterface|CreateWidget "/Game/Blueprints/PopUpScreens/FourthTutorialScreen.FourthTutorialScreen_C"))
  (bind _output_get (Variables|Default|SetFourthTutorialScreen _returnvalue))
  (UserInterface|Viewport|AddtoViewport _output_get 0))

(event EventFirstTreePlanted
  (bind _fourthtutorialscreen (Variables|Default|GetFourthTutorialScreen))
  (Utilities|IsValid _fourthtutorialscreen
    (:Is%20Valid
      (Default|CallFirstTreePlanted _fourthtutorialscreen))))

(event EventFinishedShootingPractice
  (CallFunction|RemoveTutorialWidgets)
  (bind _returnvalue (UserInterface|CreateWidget "/Game/Blueprints/PopUpScreens/FifthTutorialScreen.FifthTutorialScreen_C"))
  (bind _output_get (Variables|Default|SetFifthTutorialScreen _returnvalue))
  (UserInterface|Viewport|AddtoViewport _output_get 0))

(event EventEnteredHordeZone
  (CallFunction|RemoveTutorialWidgets)
  (bind _returnvalue (UserInterface|CreateWidget "/Game/Blueprints/PopUpScreens/SixthTutorialScreen.SixthTutorialScreen_C"))
  (bind _output_get (Variables|Default|SetSixthTutorialScreen _returnvalue))
  (UserInterface|Viewport|AddtoViewport _output_get 0))

(event Input|KeyboardEvents|P
  (params (Key :type Key%20Structure :default "None"))
  (bind _returnvalue (Game|GetPlayerController 0))
  (bind _returnvalue_2 (Game|GetPlayerController 0))
  (:Pressed
    (if (Game|IsGamePaused)
      (Variables|/Script/Engine.PlayerController|SetbShowMouseCursor _returnvalue false)
      (Input|SetInputModeGameOnly _returnvalue)
      (Widget|RemovefromParent (Variables|Default|GetPauseMenu))
      (Widget|SetVisibility (Variables|Default|GetHUD) "Visible")
      (Game|SetGamePaused false)
      (else
        (Utilities|IsValid (Variables|Default|GetPauseMenu)
          (:Is%20Valid
            _)
          (:Is%20Not%20Valid
            (bind _returnvalue_3 (UserInterface|CreateWidget "/Game/Blueprints/Menus/PauseMenu.PauseMenu_C"))
            (Variables|Default|SetPauseMenu _returnvalue_3)))
        (Variables|/Script/Engine.PlayerController|SetbShowMouseCursor _returnvalue_2 true)
        (UserInterface|Viewport|AddtoViewport (Variables|Default|GetPauseMenu) 0)
        (Input|SetInputModeGameandUI _returnvalue_2 (Variables|Default|GetPauseMenu) "DoNotLock" true)
        (Widget|SetVisibility (Variables|Default|GetHUD) "Hidden")
        (Game|SetGamePaused true)))))

(fn ConstructionScript)