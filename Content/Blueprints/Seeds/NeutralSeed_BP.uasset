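; NeutralSeed_BP is a seed that shows an indicator while it is the player koala's sighted neutral seed.
; It caches the player's KoalaCharacter_BP on BeginPlay.
; Each Tick it reads the koala's NeutralSeedOnSight flag and NeutralSeed reference, showing the Indicator only when the flag is set and the reference is itself.
; Visibility is changed only when the state differs, and detection itself happens outside this Blueprint.
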(event EventBeginPlay
  (bind _askoala_character_bp (Utilities|Casting|CastToKoalaCharacter_BP (Game|GetPlayerCharacter 0)))
  (Variables|Default|SetKoala _askoala_character_bp))

(event EventTick
  (params (DeltaSeconds :type Float%20%28single-precision%29))
  (bind _koala (Variables|Default|GetKoala))
  (bind _indicator (Variables|Default|GetIndicator))
  (bind _indicator_2 (Variables|Default|GetIndicator))
  (bind _returnvalue (Rendering|IsVisible _indicator))
  (Utilities|IsValid _koala
    (:Is%20Valid
      (if (and (Variables|/Script/Koala.KoalaCharacter|GetbNeutralSeedOnSight _koala) (== (Variables|/Script/Koala.KoalaCharacter|GetNeutralSeed _koala) self))
        (if (not _returnvalue)
          (Rendering|SetVisibility _indicator_2 true false))
        (elif _returnvalue
          (Rendering|SetVisibility _indicator_2 false false))))))

(fn ConstructionScript)