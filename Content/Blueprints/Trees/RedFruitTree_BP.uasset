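; RedFruitTree_BP is a red fruit tree actor that shows a pulp bar widget when the koala player is near.
; On BeginPlay it caches the player's KoalaCharacter_BP, creates a TreePulp widget for its PulpBar component, and passes itself to that widget as RedTree.
; Each tick it toggles the bar's visibility by whether the koala is within a fixed distance.
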(event EventBeginPlay
  (bind _pulpbar (Variables|Default|GetPulpBar))
  (bind _askoala_character_bp (Utilities|Casting|CastToKoalaCharacter_BP (Game|GetPlayerCharacter 0)))
  (Variables|Default|SetKoala _askoala_character_bp)
  (bind _returnvalue (UserInterface|CreateWidget "/Game/Blueprints/Trees/TreePulp.TreePulp_C"))
  (UserInterface|SetWidget _pulpbar _returnvalue)
  (bind _astree_pulp (Utilities|Casting|CastToTreePulp (UserInterface|GetUserWidgetObject _pulpbar)))
  (Variables|/Game/Blueprints/Trees/TreePulp.TreePulp_C|SetRedTree _astree_pulp self))

(event EventTick
  (params (DeltaSeconds :type Float%20%28single-precision%29))
  (Rendering|SetVisibility (Variables|Default|GetPulpBar) (< (Transformation|GetDistanceTo (Variables|Default|GetKoala)) 1.25e+03) false))

(fn ConstructionScript)