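; Neutral tree Blueprint that carries an HP bar widget component.
; On BeginPlay it creates a NeutralTreeHP widget, assigns it to the HPBar component and gives the widget a reference back to this tree.
; Each Tick it syncs the bar's visibility with the ShowHPBar flag, changing it only when the two differ.
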(event EventBeginPlay
  (bind _hpbar (Variables|Default|GetHPBar))
  (bind _returnvalue (UserInterface|CreateWidget "/Game/Blueprints/Trees/NeutralTreeHP.NeutralTreeHP_C"))
  (UserInterface|SetWidget _hpbar _returnvalue)
  (bind _asneutral_tree_hp (Utilities|Casting|CastToNeutralTreeHP (UserInterface|GetUserWidgetObject _hpbar)))
  (Variables|/Game/Blueprints/Trees/NeutralTreeHP.NeutralTreeHP_C|SetNeutralTree _asneutral_tree_hp self))

(event EventTick
  (params (DeltaSeconds :type Float%20%28single-precision%29))
  (bind _hpbar (Variables|Default|GetHPBar))
  (bind _hpbar_2 (Variables|Default|GetHPBar))
  (bind _returnvalue (Rendering|IsVisible _hpbar))
  (if (Variables|Default|GetbShowHPBar)
    (if (not _returnvalue)
      (Rendering|SetVisibility _hpbar_2 true false))
    (elif _returnvalue
      (Rendering|SetVisibility _hpbar_2 false false))))

(fn ConstructionScript)