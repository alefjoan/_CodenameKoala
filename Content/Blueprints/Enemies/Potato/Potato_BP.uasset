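; Potato enemy actor with a floating HP bar widget, a red "mad" look and optional moving-dummy modes.
; BeginPlay links the EnemyHP widget to itself and caches the player koala, whose distance toggles bar visibility on Tick.
; Middle and back dummies shuttle along world Y on Tick at different per-frame steps, reversing only at exact hard-coded positions.
; PotatoDeath destroys the bar and turns the mesh into a world-only physics object.
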(event EventBeginPlay
  (bind _askoala_character_bp (Utilities|Casting|CastToKoalaCharacter_BP (Game|GetPlayerCharacter 0)))
  (Variables|Default|SetKoalaLocator _askoala_character_bp)
  (bind _returnvalue (UserInterface|CreateWidget "/Game/Blueprints/Enemies/Potato/EnemyHP.EnemyHP_C"))
  (UserInterface|SetWidget (Variables|Default|GetHPBar) _returnvalue)
  (bind _asenemy_hp (Utilities|Casting|CastToEnemyHP (UserInterface|GetUserWidgetObject (Variables|Default|GetHPBar))))
  (Variables|/Game/Blueprints/Enemies/Potato/EnemyHP.EnemyHP_C|SetPotato _asenemy_hp self))

(event EventTick
  (params (DeltaSeconds :type Float%20%28single-precision%29))
  (bind _returnvalue (Transformation|GetActorLocation))
  (bind _returnvalue_2 (Transformation|GetActorLocation))
  (bind _returnvalue_3 (Transformation|GetActorLocation))
  (bind _returnvalue_4 (Transformation|GetActorLocation))
  (bind _returnvalue_5 (Transformation|GetActorLocation))
  (bind _returnvalue_6 (Transformation|GetActorLocation))
  (bind _returnvalue_7 (Transformation|GetActorLocation))
  (bind _returnvalue_8 (Transformation|GetActorLocation))
  (bind _staticmesh (Variables|Default|GetStaticMesh))
  (bind _hpbar (Variables|Default|GetHPBar))
  (Utilities|FlowControl|Sequence
    (:then_0
      (Utilities|IsValid (Variables|Default|GetHPBar)
        (:Is%20Valid
          (if (< (Transformation|GetDistanceTo (Variables|Default|GetKoalaLocator)) 2e+03)
            (Rendering|SetVisibility _hpbar true false)
            (else
              (Rendering|SetVisibility _hpbar false false))))))
    (:then_1
      (if (Variables|Default|GetbMadPotato)
        (Rendering|Material|SetMaterial _staticmesh 8 "/Game/Mats/Red.Red")
        (Rendering|Material|SetMaterial _staticmesh 0 "/Game/Mats/Red.Red")))
    (:then_2
      (if (Variables|Default|GetbMiddleDummy)
        (Utilities|FlowControl|Sequence
          (:then_0
            (if (Math|Vector|Equal(Vector) (Transformation|GetActorLocation) (Math|Vector|MakeVector (.x _returnvalue_8) -2.4e+03 (.z _returnvalue_8)) 0.0)
              (Variables|Default|SetReverseMove true)
              (Variables|Default|SetMove false)))
          (:then_1
            (if (Math|Vector|Equal(Vector) (Transformation|GetActorLocation) (Math|Vector|MakeVector (.x _returnvalue_7) -7e+01 (.z _returnvalue_7)) 0.0)
              (Variables|Default|SetMove true)
              (Variables|Default|SetReverseMove false)))
          (:then_2
            (if (Variables|Default|GetMove)
              (Transformation|SetActorLocation (Math|Vector|MakeVector (.x _returnvalue_6) (- (.y _returnvalue_6) 1e+01) (.z _returnvalue_6)) true false)))
          (:then_3
            (if (Variables|Default|GetReverseMove)
              (Transformation|SetActorLocation (Math|Vector|MakeVector (.x _returnvalue_5) (+ (.y _returnvalue_5) 1e+01) (.z _returnvalue_5)) true false))))))
    (:then_3
      (if (Variables|Default|GetbBackDummy)
        (Utilities|FlowControl|Sequence
          (:then_0
            (if (Math|Vector|Equal(Vector) (Transformation|GetActorLocation) (Math|Vector|MakeVector (.x _returnvalue_2) -2.4e+03 (.z _returnvalue_2)) 0.0)
              (Variables|Default|SetReverseMove true)
              (Variables|Default|SetMove false)))
          (:then_1
            (if (Math|Vector|Equal(Vector) (Transformation|GetActorLocation) (Math|Vector|MakeVector (.x _returnvalue_4) -7e+01 (.z _returnvalue_4)) 0.0)
              (Variables|Default|SetMove true)
              (Variables|Default|SetReverseMove false)))
          (:then_2
            (if (Variables|Default|GetMove)
              (Transformation|SetActorLocation (Math|Vector|MakeVector (.x _returnvalue) (- (.y _returnvalue) 5.0) (.z _returnvalue)) true false)))
          (:then_3
            (if (Variables|Default|GetReverseMove)
              (Transformation|SetActorLocation (Math|Vector|MakeVector (.x _returnvalue_3) (+ (.y _returnvalue_3) 5.0) (.z _returnvalue_3)) true false))))))))

(event EventPotatoDeath
  (bind _staticmesh (Variables|Default|GetStaticMesh))
  (bind _hpbar (Variables|Default|GetHPBar))
  (Utilities|FlowControl|Sequence
    (:then_0
      (Utilities|IsValid _hpbar
        (:Is%20Valid
          (Components|DestroyComponent _hpbar))))
    (:then_1
      (Collision|SetCollisionProfileName _staticmesh "WorldOnly" true :!class /Script/Engine.PrimitiveComponent)
      (Physics|SetSimulatePhysics _staticmesh true))))

(fn ConstructionScript)